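; Radio actor that switches its audio on and off each time it takes damage.
; AnyDamage drives a FlipFlop that sets the Playing flag and calls the Radio event.
; That event either spawns and activates a new non-spatial 2D sound, or deactivates the spawned audio component, so playback restarts rather than resumes.
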(event Custom|Radio
  (if (Variables|Default|GetPlaying?)
    (bind _returnvalue (Audio|SpawnSound2D "/Game/Dil/Audio/Radio.Radio" 1.0 1.0 0.0 0))
    (Components|Activation|SetActive _returnvalue true false)
    (else
      (Components|Activation|Deactivate _returnvalue))))

(event Game|Damage|EventAnyDamage
  (params (Damage :type Float%20%28single-precision%29) (DamageType :type Damage%20Type%20Object%20Reference) (InstigatedBy :type Controller%20Object%20Reference) (DamageCauser :type Actor%20Object%20Reference))
  (Utilities|FlowControl|FlipFlop
    (:A
      (Variables|Default|SetPlaying? true)
      (CallFunction|Radio))
    (:B
      (Variables|Default|SetPlaying? false)
      (CallFunction|Radio))))

(fn ConstructionScript)